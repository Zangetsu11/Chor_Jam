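; BP_Note1 is a note object that shows the WB_Note1 widget on screen when interacted with.
; Its DoorInteract event uses a FlipFlop to alternate between opening and closing the note, playing a button-push sound at the Cube each time.
; Opening creates the widget and blocks the player's look and move input, while closing removes it and restores input.
; The separate Interact function is a stub that returns false.
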(event EventDoorInteract
  (bind _returnvalue (Game|GetPlayerController 0))
  (bind _cube (Variables|Default|GetCube))
  (bind _returnvalue_2 (Transformation|GetWorldLocation _cube))
  (Utilities|FlowControl|FlipFlop
    (:A
      (Audio|PlaySoundatLocation "/Game/Audio/Cues/Cue_PushButton.Cue_PushButton" _returnvalue_2 "0, 0, 0" 1.0 1.0 0.0 0 0 0 0)
      (bind _returnvalue_3 (UserInterface|CreateWidget "/Game/Blueprints/Note/WB_Note1.WB_Note1_C"))
      (UserInterface|Viewport|AddtoViewport _returnvalue_3 0)
      (Input|SetIgnoreLookInput _returnvalue true)
      (Input|SetIgnoreMoveInput _returnvalue true))
    (:B
      (Audio|PlaySoundatLocation "/Game/Audio/Cues/Cue_PushButton.Cue_PushButton" _returnvalue_2 "0, 0, 0" 1.0 1.0 0.0 0 0 0 0)
      (Widget|RemovefromParent _returnvalue_3)
      (Input|SetIgnoreLookInput _returnvalue false)
      (Input|SetIgnoreMoveInput _returnvalue false))))

(fn ConstructionScript)

(fn Interact
  (params (Interactor :type Character%20Object%20Reference))
  (return false))
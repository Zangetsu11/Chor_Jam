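; BP_Note is an interactable note actor that shows a WB_Note widget on screen.
; The DoorInteract event feeds a FlipFlop whose A branch plays a button sound at the Cube, creates the widget and locks the player's look and move input.
; The B branch is unwired, and the logic that removes the widget and restores input is disconnected.
; The separate Interact function only returns false.
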(event EventDoorInteract
  (bind _returnvalue (Game|GetPlayerController 0))
  (Utilities|FlowControl|FlipFlop
    (:A
      (Audio|PlaySoundatLocation "/Game/Audio/Cues/Cue_PushButton.Cue_PushButton" (Transformation|GetWorldLocation (Variables|Default|GetCube)) "0, 0, 0" 1.0 1.0 0.0 0 0 0 0)
      (bind _returnvalue_2 (UserInterface|CreateWidget "/Game/Blueprints/Note/WB_Note.WB_Note_C"))
      (UserInterface|Viewport|AddtoViewport _returnvalue_2 0)
      (Input|SetIgnoreLookInput _returnvalue true)
      (Input|SetIgnoreMoveInput _returnvalue true))))

(fn ConstructionScript)

(fn Interact
  (params (Interactor :type Character%20Object%20Reference))
  (return false))
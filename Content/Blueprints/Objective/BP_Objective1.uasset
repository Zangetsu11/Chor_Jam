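; Placeable objective trigger that announces an objective to the player through an on-screen Objective_Widget.
; The widget is created at BeginPlay, then shown once when the player character overlaps the box (sized in the Construction Script), with sound and a timed fade in and out.
; A CompletedObjective event reuses that widget to announce completion.
; Both announcements set ObjectiveInProgress to true after their delayed fade-out starts.
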(event OnComponentBeginOverlap(Objective_Box)
  (params (OverlappedComponent :type Primitive%20Component%20Object%20Reference) (OtherActor :type Actor%20Object%20Reference) (OtherComp :type Primitive%20Component%20Object%20Reference) (OtherBodyIndex :type Integer) (bFromSweep :type Boolean) (SweepResult :type Hit%20Result%20Structure%20%28by%20ref%29))
  (bind _objective_ref (Variables|Default|GetObjective_Ref))
  (bind _objective_ref_2 (Variables|Default|GetObjective_Ref))
  (bind _fade (Variables|/Game/Widgets/Objective_Widget.Objective_Widget_C|GetFade _objective_ref))
  (if (== OtherActor (Game|GetPlayerCharacter 0))
    (Utilities|FlowControl|DoOnce false
      (:Completed
        (Variables|/Game/Widgets/Objective_Widget.Objective_Widget_C|SetObj_Title_Text _objective_ref_2 (Variables|Default|GetObjective%20Title%20Text))
        (Variables|/Game/Widgets/Objective_Widget.Objective_Widget_C|SetObj_Info_Text _objective_ref_2 (Variables|Default|GetObjective%20Content%20Text))
        (Appearance|SetColorandOpacity (Variables|/Game/Widgets/Objective_Widget.Objective_Widget_C|GetObjective_Info _objective_ref_2) (Utilities|Struct|MakeSlateColor (Utilities|Struct|MakeLinearColor 1.0 0.0 1.0 1.0) "UseColor_Specified") :!class /Script/UMG.TextBlock)
        (Audio|PlaySound2D "/Game/Audio/Cues/Objective.Objective" 1.0 1.0 0.0 0 0)
        (UserInterface|Viewport|AddtoViewport _objective_ref 0)
        (UserInterface|Animation|PlayAnimation _objective_ref _fade 0.0 1 "Forward" 1.0 false)
        (Utilities|FlowControl|Delay 5.0)
        (UserInterface|Animation|PlayAnimation _objective_ref _fade 0.0 1 "Reverse" 1.0 false)
        (Variables|Default|SetObjective%20In%20Progress%20? true)))))

(event Custom|Completed%20Objective
  (bind _objective_ref (Variables|Default|GetObjective_Ref))
  (bind _objective_ref_2 (Variables|Default|GetObjective_Ref))
  (bind _fade (Variables|/Game/Widgets/Objective_Widget.Objective_Widget_C|GetFade _objective_ref))
  (Variables|/Game/Widgets/Objective_Widget.Objective_Widget_C|SetObj_Title_Text _objective_ref_2 "Completed Objective")
  (Appearance|SetColorandOpacity (Variables|/Game/Widgets/Objective_Widget.Objective_Widget_C|GetObjective_Info _objective_ref_2) (Utilities|Struct|MakeSlateColor (Utilities|Struct|MakeLinearColor 1.0 0.0 1.0 1.0) "UseColor_Specified") :!class /Script/UMG.TextBlock)
  (Audio|PlaySound2D 0 1.0 1.0 0.0 0 0)
  (UserInterface|Animation|PlayAnimation _objective_ref _fade 0.0 1 "Forward" 1.0 false)
  (Utilities|FlowControl|Delay 3.0)
  (UserInterface|Animation|PlayAnimation _objective_ref _fade 0.0 1 "Reverse" 1.0 false)
  (Variables|Default|SetObjective%20In%20Progress%20? true))

(event EventBeginPlay
  (bind _returnvalue (UserInterface|CreateWidget "/Game/Widgets/Objective_Widget.Objective_Widget_C" 0 (Variables|Default|GetObjective%20Title%20Text) (Variables|Default|GetObjective%20Content%20Text)))
  (Variables|Default|SetObjective_Ref _returnvalue))

(fn ConstructionScript
  (Components|Box|SetBoxExtent (Variables|Default|GetObjective_Box) (Variables|Default|GetObjective%20Box%20Size) true))
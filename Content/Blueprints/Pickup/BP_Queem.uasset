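; BP_Queem is an interactable pickup that shows an objective notification when the player uses it.
; A Box trigger shows and hides an interact prompt widget for the player.
; Interact plays a coin sound and destroys the actor after a short delay, while a once-only event fades in the objective widget.
; That event's delayed fade-out outlasts the actor's destruction delay, and the overlap pickup counter adds zero.
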(event OnComponentBeginOverlap(Box)
  (params (OverlappedComponent :type Primitive%20Component%20Object%20Reference) (OtherActor :type Actor%20Object%20Reference) (OtherComp :type Primitive%20Component%20Object%20Reference) (OtherBodyIndex :type Integer) (bFromSweep :type Boolean) (SweepResult :type Hit%20Result%20Structure%20%28by%20ref%29))
  ;[1 1 1] Press to Interact
  (if (== OtherActor (Game|GetPlayerCharacter 0))
    (UserInterface|Viewport|AddtoViewport (Variables|Default|GetInteractPrompt) 0)))

(event OnComponentEndOverlap(Box)
  (params (OverlappedComponent :type Primitive%20Component%20Object%20Reference) (OtherActor :type Actor%20Object%20Reference) (OtherComp :type Primitive%20Component%20Object%20Reference) (OtherBodyIndex :type Integer))
  ;[1 1 1] Press to Interact
  (if (== (Game|GetPlayerCharacter 0) OtherActor)
    (Widget|RemovefromParent (Variables|Default|GetInteractPrompt))))

(event Custom|DestroyItem
  ;[1 1 1] Remove Item
  (Utilities|FlowControl|Delay 0.2)
  (Audio|PlaySoundatLocation "/Game/Audio/Cues/Coin.Coin" (Transformation|GetWorldLocation (Variables|Default|GetItem)) "0, 0, 0" 1.0 1.0 0.0 0 0 0 0)
  (Actor|DestroyActor))

(event Custom|Objective
  (bind _objective_ref (Variables|Default|GetObjective_Ref))
  (bind _objective_ref_2 (Variables|Default|GetObjective_Ref))
  (bind _objective_ref_3 (Variables|Default|GetObjective_Ref))
  (Utilities|FlowControl|DoOnce false
    (:Completed
      (Variables|/Game/Widgets/Objective_Widget.Objective_Widget_C|SetObj_Title_Text _objective_ref_3 (Variables|Default|GetObjective%20Title%20Text))
      (Variables|/Game/Widgets/Objective_Widget.Objective_Widget_C|SetObj_Info_Text _objective_ref_3 (Variables|Default|GetObjective%20Content%20Text))
      (Appearance|SetColorandOpacity (Variables|/Game/Widgets/Objective_Widget.Objective_Widget_C|GetObjective_Info _objective_ref_3) (Utilities|Struct|MakeSlateColor (Utilities|Struct|MakeLinearColor 1.0 0.0 1.0 1.0) "UseColor_Specified") :!class /Script/UMG.TextBlock)
      (Audio|PlaySound2D "/Game/Audio/Cues/Objective.Objective" 1.0 1.0 0.0 0 0)
      (UserInterface|Viewport|AddtoViewport _objective_ref 0)
      (UserInterface|Animation|PlayAnimation _objective_ref (Variables|/Game/Widgets/Objective_Widget.Objective_Widget_C|GetFade _objective_ref) 0.0 1 "Forward" 1.0 false)
      (Utilities|FlowControl|Delay 1.0)
      (UserInterface|Animation|PlayAnimation _objective_ref_2 (Variables|/Game/Widgets/Objective_Widget.Objective_Widget_C|GetFade _objective_ref_2) 0.0 1 "Reverse" 1.0 false)
      (Variables|Default|SetObjective%20In%20Progress%20? true))))

(event EventBeginPlay
  ;[1 1 1] Press to Interact
  (bind _returnvalue (UserInterface|CreateWidget "/Game/Blueprints/Door/Interact_Widget.Interact_Widget_C"))
  (Variables|Default|SetInteractPrompt _returnvalue)
  (bind _returnvalue_2 (UserInterface|CreateWidget "/Game/Widgets/Objective_Widget.Objective_Widget_C" 0 (Variables|Default|GetObjective%20Title%20Text) (Variables|Default|GetObjective%20Content%20Text)))
  (Variables|Default|SetObjective_Ref _returnvalue_2))

(event Collision|EventActorBeginOverlap
  (params (OtherActor :type Actor%20Object%20Reference))
  ;[1 1 1] Pick Item
  (Utilities|FlowControl|DoOnce (Variables|Default|Getpicked%20?)
    (:Completed
      (bind _asbp_third_person_character (Utilities|Casting|CastToBP_ThirdPersonCharacter OtherActor))
      (Variables|/Game/ThirdPerson/Blueprints/BP_ThirdPersonCharacter.BP_ThirdPersonCharacter_C|SetPickupAmount _asbp_third_person_character (+ (Variables|/Game/ThirdPerson/Blueprints/BP_ThirdPersonCharacter.BP_ThirdPersonCharacter_C|GetPickupAmount _asbp_third_person_character) 0)))))

(fn ConstructionScript)

(fn Interact
  (params (Interactor :type Character%20Object%20Reference))
  ;[1 1 1] Interact System
  (CallFunction|DestroyItem)
  (CallFunction|Objective)
  (return false))
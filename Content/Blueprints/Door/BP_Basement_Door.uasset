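; BP_Basement_Door is an interactable door that plays a level sequence and moves the player to a spawn location.
; A box overlap shows and hides an interact prompt widget for the player character.
; Interact fires SpawnPlayer, which hides the player, plays the sequence, waits a fixed delay, then unhides and relocates the player.
; The delay is hard-coded rather than tied to the sequence finishing.
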(event OnComponentBeginOverlap(Box)
  (params (OverlappedComponent :type Primitive%20Component%20Object%20Reference) (OtherActor :type Actor%20Object%20Reference) (OtherComp :type Primitive%20Component%20Object%20Reference) (OtherBodyIndex :type Integer) (bFromSweep :type Boolean) (SweepResult :type Hit%20Result%20Structure%20%28by%20ref%29))
  ;[1 1 1] Press to Interact
  (if (== OtherActor (Game|GetPlayerCharacter 0))
    (UserInterface|Viewport|AddtoViewport (Variables|Default|GetInteractPrompt) 0)))

(event OnComponentEndOverlap(Box)
  (params (OverlappedComponent :type Primitive%20Component%20Object%20Reference) (OtherActor :type Actor%20Object%20Reference) (OtherComp :type Primitive%20Component%20Object%20Reference) (OtherBodyIndex :type Integer))
  ;[1 1 1] Press to Interact
  (if (== (Game|GetPlayerCharacter 0) OtherActor)
    (Widget|RemovefromParent (Variables|Default|GetInteractPrompt))))

(event Custom|Spawn%20Player
  (bind _returnvalue (Game|GetPlayerCharacter 0))
  (Rendering|SetActorHiddenInGame _returnvalue true)
  (bind _outactor (Sequencer|Player|CreateLevelSequencePlayer "/Game/Animations/NewLevelSequence.NewLevelSequence"))
  (Sequencer|Player|Play (Variables|/Script/LevelSequence.LevelSequenceActor|GetSequencePlayer _outactor) :!class /Script/MovieScene.MovieSceneSequencePlayer)
  (Utilities|FlowControl|Delay 3.0)
  (Rendering|SetActorHiddenInGame _returnvalue false)
  (Transformation|SetActorLocation _returnvalue (Variables|Default|GetSpawn%20Transform%20Location) false false))

(event EventBeginPlay
  ;[1 1 1] Press to Interact
  (bind _returnvalue (UserInterface|CreateWidget "/Game/Blueprints/Door/Interact_Widget.Interact_Widget_C"))
  (Variables|Default|SetInteractPrompt _returnvalue))

(fn ConstructionScript)

(fn Interact
  (params (Interactor :type Character%20Object%20Reference))
  ;[1 1 1] Open Door
  (CallFunction|SpawnPlayer)
  (return true))
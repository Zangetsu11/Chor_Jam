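; Key-locked door that swings open on interaction once PickUpKey has set HasKey.
; Interact calls Open, where a FlipFlop with only A wired plays a timeline lerping door yaw; nothing closes it.
; A box overlap shows or hides the player's interact prompt.
; Without the key, Objective shows a one-time fading objective with sound, though the code creating its widget is disconnected here.
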(event OnComponentBeginOverlap(Box)
  (params (OverlappedComponent :type Primitive%20Component%20Object%20Reference) (OtherActor :type Actor%20Object%20Reference) (OtherComp :type Primitive%20Component%20Object%20Reference) (OtherBodyIndex :type Integer) (bFromSweep :type Boolean) (SweepResult :type Hit%20Result%20Structure%20%28by%20ref%29))
  ;[1 1 1] Press to Interact
  (if (== OtherActor (Game|GetPlayerCharacter 0))
    (UserInterface|Viewport|AddtoViewport (Variables|Default|GetInteractPrompt) 0)))

(event OnComponentEndOverlap(Box)
  (params (OverlappedComponent :type Primitive%20Component%20Object%20Reference) (OtherActor :type Actor%20Object%20Reference) (OtherComp :type Primitive%20Component%20Object%20Reference) (OtherBodyIndex :type Integer))
  ;[1 1 1] Press to Interact
  (if (== (Game|GetPlayerCharacter 0) OtherActor)
    (Widget|RemovefromParent (Variables|Default|GetInteractPrompt))))

(event Custom|Open
  ;[1 1 1] Key ?
  (if (Variables|Default|GetHas%20Key?)
    (Utilities|FlowControl|FlipFlop
      (:A
        (bind _movement (Timeline|Door%20Timeline Play)
          (:Update
            (Transformation|SetRelativeRotation (Variables|Default|GetDoor) (Math|Rotator|MakeRotator 0.0 0.0 (Math|Float|Lerp 0.0 -9e+01 _movement)) false false)))))))

(event Custom|Objective
  (bind _objective_ref (Variables|Default|GetObjective_Ref))
  (bind _objective_ref_2 (Variables|Default|GetObjective_Ref))
  (bind _fade (Variables|/Game/Widgets/Objective_Widget.Objective_Widget_C|GetFade _objective_ref))
  (if (not (Variables|Default|GetHas%20Key?))
    (Utilities|FlowControl|DoOnce false
      (:Completed
        (Variables|/Game/Widgets/Objective_Widget.Objective_Widget_C|SetObj_Title_Text _objective_ref_2 (Variables|Default|GetObjective%20Title%20Text))
        (Variables|/Game/Widgets/Objective_Widget.Objective_Widget_C|SetObj_Info_Text _objective_ref_2 (Variables|Default|GetObjective%20Content%20Text))
        (Appearance|SetColorandOpacity (Variables|/Game/Widgets/Objective_Widget.Objective_Widget_C|GetObjective_Info _objective_ref_2) (Utilities|Struct|MakeSlateColor (Utilities|Struct|MakeLinearColor 1.0 0.0 1.0 1.0) "UseColor_Specified") :!class /Script/UMG.TextBlock)
        (Audio|PlaySound2D "/Game/Audio/Cues/Objective.Objective" 1.0 1.0 0.0 0 0)
        (UserInterface|Viewport|AddtoViewport _objective_ref 0)
        (UserInterface|Animation|PlayAnimation _objective_ref _fade 0.0 1 "Forward" 1.0 false)
        (Utilities|FlowControl|Delay 5.0)
        (UserInterface|Animation|PlayAnimation _objective_ref _fade 0.0 1 "Reverse" 1.0 false)))))

(event EventBeginPlay
  ;[1 1 1] Press to Interact
  (bind _returnvalue (UserInterface|CreateWidget "/Game/Blueprints/Door/Interact_Widget.Interact_Widget_C"))
  (Variables|Default|SetInteractPrompt _returnvalue))

(event EventPickUpKey
  ;[1 1 1] Key ?
  (Variables|Default|SetHas%20Key? true))

(fn ConstructionScript)

(fn Interact
  (params (Interactor :type Character%20Object%20Reference))
  ;[1 1 1] Open Door with key
  (if (Variables|Default|GetHas%20Key?)
    (CallFunction|Open)
    (return true)))
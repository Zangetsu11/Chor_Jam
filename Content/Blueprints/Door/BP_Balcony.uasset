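; BP_Balcony is an interactable balcony door that stays locked until its PickUpKey event sets HasKey.
; Interact checks the key and calls Open, where a FlipFlop alternately plays and reverses a timeline that swings the door's yaw up to 100 degrees.
; An Interact_Widget prompt, created on BeginPlay, shows while the player character overlaps the Box trigger.
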(event OnComponentBeginOverlap(Box)
  (params (OverlappedComponent :type Primitive%20Component%20Object%20Reference) (OtherActor :type Actor%20Object%20Reference) (OtherComp :type Primitive%20Component%20Object%20Reference) (OtherBodyIndex :type Integer) (bFromSweep :type Boolean) (SweepResult :type Hit%20Result%20Structure%20%28by%20ref%29))
  ;[1 1 1] Press to Interact
  (if (== OtherActor (Game|GetPlayerCharacter 0))
    (UserInterface|Viewport|AddtoViewport (Variables|Default|GetInteractPrompt) 0)))

(event OnComponentEndOverlap(Box)
  (params (OverlappedComponent :type Primitive%20Component%20Object%20Reference) (OtherActor :type Actor%20Object%20Reference) (OtherComp :type Primitive%20Component%20Object%20Reference) (OtherBodyIndex :type Integer))
  ;[1 1 1] Press to Interact
  (if (== (Game|GetPlayerCharacter 0) OtherActor)
    (Widget|RemovefromParent (Variables|Default|GetInteractPrompt))))

(event Custom|Open
  ;[1 1 1] Key ?
  (if (Variables|Default|GetHas%20Key?)
    (Utilities|FlowControl|FlipFlop
      (:A
        (bind _movement (Timeline|Door%20Timeline Play)
          (:Update
            (Transformation|SetRelativeRotation (Variables|Default|GetDoor) (Math|Rotator|MakeRotator 0.0 0.0 (Math|Float|Lerp 0.0 -1e+02 _movement)) false false))))
      (:B
        (Timeline|Door%20Timeline Reverse)))))

(event EventBeginPlay
  ;[1 1 1] Press to Interact
  (bind _returnvalue (UserInterface|CreateWidget "/Game/Blueprints/Door/Interact_Widget.Interact_Widget_C"))
  (Variables|Default|SetInteractPrompt _returnvalue))

(event EventPickUpKey
  ;[1 1 1] Key ?
  (Variables|Default|SetHas%20Key? true))

(fn ConstructionScript)

(fn Interact
  (params (Interactor :type Character%20Object%20Reference))
  ;[1 1 1] Open Door with key
  (if (Variables|Default|GetHas%20Key?)
    (CallFunction|Open)
    (return true)))
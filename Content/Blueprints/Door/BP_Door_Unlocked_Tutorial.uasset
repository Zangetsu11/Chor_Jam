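; Tutorial door Blueprint that, when interacted with, plays a storyline sequence and then moves the game to the Demonstration_Map level.
; An overlap box shows an interact prompt widget, created at BeginPlay, while the player character is inside it.
; Interact triggers the widget animation event, which adds a Storyline widget, plays its Story animation and opens the level after a fixed delay rather than on animation completion.
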(event OnComponentBeginOverlap(Box)
  (params (OverlappedComponent :type Primitive%20Component%20Object%20Reference) (OtherActor :type Actor%20Object%20Reference) (OtherComp :type Primitive%20Component%20Object%20Reference) (OtherBodyIndex :type Integer) (bFromSweep :type Boolean) (SweepResult :type Hit%20Result%20Structure%20%28by%20ref%29))
  ;[1 1 1] Press to Interact
  (if (== OtherActor (Game|GetPlayerCharacter 0))
    (UserInterface|Viewport|AddtoViewport (Variables|Default|GetInteractPrompt) 0)))

(event OnComponentEndOverlap(Box)
  (params (OverlappedComponent :type Primitive%20Component%20Object%20Reference) (OtherActor :type Actor%20Object%20Reference) (OtherComp :type Primitive%20Component%20Object%20Reference) (OtherBodyIndex :type Integer))
  ;[1 1 1] Press to Interact
  (if (== (Game|GetPlayerCharacter 0) OtherActor)
    (Widget|RemovefromParent (Variables|Default|GetInteractPrompt))))

(event Custom|Widget_Animation
  ;[1 1 1] Widget Animation
  (bind _returnvalue (UserInterface|CreateWidget "/Game/Widgets/2DCutScene/Storyline.Storyline_C"))
  (Variables|Default|SetNewVar_0 _returnvalue)
  (UserInterface|Viewport|AddtoViewport (Variables|Default|GetNewVar_0) 0)
  (UserInterface|Animation|PlayAnimation (Variables|Default|GetNewVar_0) (Variables|/Game/Widgets/2DCutScene/Storyline.Storyline_C|GetStory (Variables|Default|GetNewVar_0)) 0.0 1 "Forward" 1.0 false)
  (Utilities|FlowControl|Delay 65.0)
  (Game|OpenLevel(byObjectReference) "/Game/Maps/Demonstration_Map.Demonstration_Map"))

(event EventBeginPlay
  ;[1 1 1] Press to Interact
  (bind _returnvalue (UserInterface|CreateWidget "/Game/Blueprints/Door/Interact_Widget.Interact_Widget_C"))
  (Variables|Default|SetInteractPrompt _returnvalue))

(fn ConstructionScript)

(fn Interact
  (params (Interactor :type Character%20Object%20Reference))
  ;[1 1 1] Teleport to New Level
  (CallFunction|WidgetAnimation)
  (return false))
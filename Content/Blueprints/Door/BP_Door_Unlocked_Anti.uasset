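; Interactable unlocked door that swings open and closed and shows an interaction prompt while the player stands in its box trigger.
; Interact plays or reverses a timeline based on IsOpen, setting the play rate from separate open and close durations.
; The timeline lerps the door's yaw between closed and open positions and flips IsOpen when it finishes.
; The prompt widget is created at BeginPlay and toggled on overlap.
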(event OnComponentBeginOverlap(Box)
  (params (OverlappedComponent :type Primitive%20Component%20Object%20Reference) (OtherActor :type Actor%20Object%20Reference) (OtherComp :type Primitive%20Component%20Object%20Reference) (OtherBodyIndex :type Integer) (bFromSweep :type Boolean) (SweepResult :type Hit%20Result%20Structure%20%28by%20ref%29))
  ;[1 1 1] Press to Interact
  (if (== OtherActor (Game|GetPlayerCharacter 0))
    (UserInterface|Viewport|AddtoViewport (Variables|Default|GetInteractPrompt) 0)))

(event OnComponentEndOverlap(Box)
  (params (OverlappedComponent :type Primitive%20Component%20Object%20Reference) (OtherActor :type Actor%20Object%20Reference) (OtherComp :type Primitive%20Component%20Object%20Reference) (OtherBodyIndex :type Integer))
  ;[1 1 1] Press to Interact
  (if (== (Game|GetPlayerCharacter 0) OtherActor)
    (Widget|RemovefromParent (Variables|Default|GetInteractPrompt))))

(event Custom|Open
  ;[1 1 1] Open/Close Door
  (bind _door_track (Timeline|Door_Time Play)
    (:Update
      (Transformation|SetRelativeRotation (Variables|Default|GetDoor) (Math|Rotator|MakeRotator 0.0 0.0 (Math|Float|Lerp (Variables|Default|GetClosePosition) (Variables|Default|GetOpenPosition) _door_track)) false false))
    (:Finished
      (Variables|Default|SetIsOpen? (not (Variables|Default|GetIsOpen?))))))

(event Custom|Close
  ;[1 1 1] Open/Close Door
  (bind _door_track (Timeline|Door_Time Reverse)
    (:Update
      (Transformation|SetRelativeRotation (Variables|Default|GetDoor) (Math|Rotator|MakeRotator 0.0 0.0 (Math|Float|Lerp (Variables|Default|GetClosePosition) (Variables|Default|GetOpenPosition) _door_track)) false false))
    (:Finished
      (Variables|Default|SetIsOpen? (not (Variables|Default|GetIsOpen?))))))

(event EventBeginPlay
  ;[1 1 1] Press to Interact
  (bind _returnvalue (UserInterface|CreateWidget "/Game/Blueprints/Door/Interact_Widget.Interact_Widget_C"))
  (Variables|Default|SetInteractPrompt _returnvalue))

(fn ConstructionScript)

(fn Interact
  (params (Interactor :type Character%20Object%20Reference))
  (bind _door_time (Variables|Default|GetDoor_Time))
  ;[1 1 1] Open Door
  (if (not (Variables|Default|GetIsOpen?))
    (Components|Timeline|SetPlayRate _door_time (/ 1.0 (Variables|Default|GetTime%20to%20open)))
    (CallFunction|Open)
    (else
      (Components|Timeline|SetPlayRate _door_time (/ 1.0 (Variables|Default|GetTime%20to%20close)))
      (CallFunction|Close)))
  (return true))
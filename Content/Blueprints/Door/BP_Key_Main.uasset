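; BP_Key_Main is a key pickup actor linked to a door.
; It creates an interact prompt widget on BeginPlay and shows or removes it as the player character enters or leaves its box trigger.
; Its Interact function notifies the referenced Door through PickUpKeyMessage, plays a sound at the mesh location, and destroys the key.
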(event OnComponentBeginOverlap(Box)
  (params (OverlappedComponent :type Primitive%20Component%20Object%20Reference) (OtherActor :type Actor%20Object%20Reference) (OtherComp :type Primitive%20Component%20Object%20Reference) (OtherBodyIndex :type Integer) (bFromSweep :type Boolean) (SweepResult :type Hit%20Result%20Structure%20%28by%20ref%29))
  ;[1 1 1] Press to Interact
  (if (== OtherActor (Game|GetPlayerCharacter 0))
    (UserInterface|Viewport|AddtoViewport (Variables|Default|GetInteractPrompt) 0)))

(event OnComponentEndOverlap(Box)
  (params (OverlappedComponent :type Primitive%20Component%20Object%20Reference) (OtherActor :type Actor%20Object%20Reference) (OtherComp :type Primitive%20Component%20Object%20Reference) (OtherBodyIndex :type Integer))
  ;[1 1 1] Press to Interact
  (if (== (Game|GetPlayerCharacter 0) OtherActor)
    (Widget|RemovefromParent (Variables|Default|GetInteractPrompt))))

(event EventBeginPlay
  ;[1 1 1] Press to Interact
  (bind _returnvalue (UserInterface|CreateWidget "/Game/Blueprints/Door/Interact_Widget.Interact_Widget_C"))
  (Variables|Default|SetInteractPrompt _returnvalue))

(fn ConstructionScript)

(fn Interact
  (params (Interactor :type Character%20Object%20Reference))
  ;[1 1 1] Pick Key
  (Class|BPIInterface|PickUpKey(Message) (Variables|Default|GetDoor))
  (Audio|PlaySoundatLocation "/Game/Audio/Wavs/S_Light.S_Light" (Transformation|GetWorldLocation (Variables|Default|GetStaticMesh)) "0, 0, 0" 1.0 1.0 0.0 0 0 0 0)
  (Actor|DestroyActor)
  (return false))